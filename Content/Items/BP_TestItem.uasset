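; BP_TestItem is a test item Blueprint whose Equipped and Unequipped events only forward to the parent class.
; BeginPlay, Tick and the construction script are empty.
; Disconnected leftover nodes hold debug prints for equipping, unequipping, entering, exiting and moving between inventory slots.
; An unused chain also fetches the owning pawn's AI controller brain as a UtilityComponent, alongside an unconnected SetUtilityComponent call.
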(event EventBeginPlay)

(event EventEquipped
  (params (OldLocation :type Inventory%20Location%20Handle%20Structure%20%28by%20ref%29))
  (|CallParentFunction OldLocation))

(event EventTick
  (params (DeltaSeconds :type Float%20%28single-precision%29)))

(event EventUnequipped
  (params (OldLocation :type Inventory%20Location%20Handle%20Structure%20%28by%20ref%29))
  (|CallParentFunction OldLocation))

(fn ConstructionScript)