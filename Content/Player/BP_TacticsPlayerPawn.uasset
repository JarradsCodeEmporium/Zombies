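; Tactics player pawn Blueprint with debug-style input for time control and unit manipulation.
; Space toggles global time dilation between zero and normal, acting as a pause.
; J traces from the world cursor, then launches each selected BaseUnit from SelectorComponent up and toward the hit point and rotates it half a turn.
; Holding T registers a delegate on WorldCursorComponent, removed by handle on release; handler functions only print test output.
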(event EventBeginPlay)

(event Collision|EventActorBeginOverlap
  (params (OtherActor :type Actor%20Object%20Reference)))

(event EventTick
  (params (DeltaSeconds :type Float%20%28single-precision%29)))

(event Input|KeyboardEvents|SpaceBar
  (params (Key :type Key%20Structure :default "None"))
  (:Pressed
    (bind _isa (Utilities|FlowControl|FlipFlop)
      (:A
        _)
      (:B
        _))
    (Utilities|Time|SetGlobalTimeDilation (Math|Float|SelectFloat 0.0 1.0 _isa))))

(event Input|MouseEvents|LeftMouseButton
  (params (Key :type Key%20Structure :default "None")))

(event Input|KeyboardEvents|J
  (params (Key :type Key%20Structure :default "None"))
  (bind _worldcursorlocation (Variables|Default|GetWorldCursorLocation))
  (:Pressed
    (bind _outhit (Collision|LineTraceByChannel (.worldlocation _worldcursorlocation) (+ (.worldlocation _worldcursorlocation) (* (.worlddirection _worldcursorlocation) 1e+04)) "TraceTypeQuery1" false 0 "ForDuration" true "(R=1.000000,G=0.000000,B=0.000000,A=1.000000)" "(R=0.000000,G=1.000000,B=0.000000,A=1.000000)" 2.0))
    (bind _result (Utilities|Set|ToArray (Variables|/Script/Zombies.GameplaySelectorComponent|GetSelectedComponents (Variables|Default|GetSelectorComponent))))
    (for _array_element _result
      (bind _asbase_unit (Utilities|Casting|CastToBaseUnit (Components|GetOwner _array_element)))
      (Character|LaunchCharacter _asbase_unit (* (+ (Class|KismetMathLibrary|VectorNormal2D (- (.location _outhit) (Transformation|GetActorLocation _asbase_unit)) 0.0001) "0,0,1.000000") 6e+02) false false)
      (Class|Actor|AddActorWorldRotation _asbase_unit "0,180.000000, 0"))))

(event Input|KeyboardEvents|T
  (params (Key :type Key%20Structure :default "None"))
  (bind _worldcursorcomponent (Variables|Default|GetWorldCursorComponent))
  (:Pressed
    (bind _returnvalue (Class|WorldCursorComponent|AddDelegate _worldcursorcomponent (EventDispatchers|CreateEvent :!event BPTacticsPlayerPawnAutoGenFunc)))
    (Variables|Default|SetHandle _returnvalue)
    (Development|PrintString "Hello"))
  (:Released
    (Class|WorldCursorComponent|RemoveDelegate _worldcursorcomponent (Variables|Default|GetHandle))))

(fn ConstructionScript)

(fn TestHandler
  (params (Params :type World%20Cursor%20Event%20Params%20Structure%20%28by%20ref%29))
  (Development|PrintString "Pawn handler" true true "(R=0.000000,G=0.660000,B=1.000000,A=1.000000)" 0.05)
  (return false))

(fn BPTacticsPlayerPawnAutoGenFunc
  (params (Params :type World%20Cursor%20Event%20Params%20Structure%20%28by%20ref%29))
  (Development|PrintText (Utilities|Text|FormatText "BP {Type} {Input}" (Utilities|String|EnumtoString (.type Params)) (Utilities|String|EnumtoString (.input Params))) false)
  (return "Captured"))