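; BP_NavLinkAbilityTest is a test ability that moves a unit across a nav link by teleporting it to the link's goal location.
; It stores the goal from the nav link params, then on begin stops movement while keeping the path.
; It teleports to the goal, raised by capsule half-height with a small random offset, retrying after a short delay until the teleport succeeds.
; A debug mesh attachment is left unconnected.
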(event EventSetFollowNavLinkParams
  (params (Params :type Follow%20Nav%20Link%20Params%20Structure%20%28by%20ref%29))
  (Variables|Default|SetGoalLocation (.goallocation Params)))

(event EventOnBeginAbility
  (bind _returnvalue (Class|Ability|GetAbilityComponent))
  (bind _returnvalue_2 (Class|AbilityComponent|GetAvatarActor _returnvalue))
  (bind _asbase_unit (Utilities|Casting|CastToBaseUnit _returnvalue_2))
  (Class|NavMovementComponent|StopMovementKeepPathing (Variables|/Script/Engine.Character|GetCharacterMovement _asbase_unit))
  (bind _returnvalue_3 (Transformation|Teleport _returnvalue_2 (+ (+ (Variables|Default|GetGoalLocation) (Math|Vector|MakeVector 0.0 0.0 (Components|Capsule|GetScaledCapsuleHalfHeight (Variables|/Script/Engine.Character|GetCapsuleComponent _asbase_unit)))) (* (Math|Random|RandomUnitVector) 1e+01)) (Transformation|GetActorRotation _asbase_unit) :!label _label)) ; teleport can fail if there's already something there
  (if (not _returnvalue_3)
    (Utilities|FlowControl|Delay 0.2)
    (goto _label)))

(fn ConstructionScript)