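; BP_ZombieDeath is an ability that handles a zombie character's death.
; When the ability begins, it casts the avatar to Character, shuts off movement and makes the capsule ignore the Pawn channel.
; It then sets a short life span so the actor is destroyed automatically and plays a death montage on the mesh.
; A debug "Dead" text draw is left unconnected and never runs.
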(event EventOnBeginAbility
  (bind _ascharacter (Utilities|Casting|CastToCharacter (Class|AbilityComponent|GetAvatarActor (Class|Ability|GetAbilityComponent))))
  (Pawn|Components|CharacterMovement|DisableMovement (Variables|/Script/Engine.Character|GetCharacterMovement _ascharacter))
  (Components|Activation|Deactivate (Variables|/Script/Engine.Character|GetCharacterMovement _ascharacter))
  (Collision|SetCollisionResponsetoChannel (Variables|/Script/Engine.Character|GetCapsuleComponent _ascharacter) "ECC_Pawn" "ECR_Ignore")
  (Actor|SetLifeSpan _ascharacter 5.0)
  (Animation|Montage|PlayMontage (Variables|/Script/Engine.Character|GetMesh _ascharacter) "/Game/Characters/Humanoid/Animations/AM_Death1.AM_Death1"))

(fn ConstructionScript)