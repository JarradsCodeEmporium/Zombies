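; Test move ability that sends an AI-controlled avatar to the location of its MoveCommand.
; An async action runs the move and its result ends the ability as Finished on success, otherwise Cancelled.
; Facing commands set a distant focal point and disable control rotation from pawn orientation, avoiding a snap to incomplete rotation when focus clears at ability end.
; The debug string drawing is disconnected.
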(event EventBeginPlay)

(event Collision|EventActorBeginOverlap
  (params (OtherActor :type Actor%20Object%20Reference)))

(event EventTick
  (params (DeltaSeconds :type Float%20%28single-precision%29)))

(event EventOnBeginAbility
  (CallFunction|SetAIController)
  (bind _asmove_command (Utilities|Casting|CastToMoveCommand (Class|Ability|GetCommand)))
  (bind _result (|TestAsyncAbilityAction "Fart" (Transformation|GetActorLocation _asmove_command))
    (:then
      (Variables|/Script/AIModule.AIController|SetbSetControlRotationFromPawnOrientation (Variables|Default|GetAIController) (Utilities|Enum|NotEqual(Enum) (Variables|/Script/Zombies.MoveCommand|GetType _asmove_command) "Facing")) ; Pathfinding move can finish before pawn is finished rotating to the desired facing.\nthis means the controller then snaps to the incomplete pawn rotation once the focus is cleared\nso we just manually set this value in here to get the desired behaviour
      (if (not (Utilities|Enum|NotEqual(Enum) (Variables|/Script/Zombies.MoveCommand|GetType _asmove_command) "Facing"))
        (AI|SetFocalPoint (Variables|Default|GetAIController) (Math|Transform|TransformLocation (Transformation|GetActorTransform _asmove_command) "999999.000000, 0, 0"))))
    (:OnMoveComplete
      (Class|Ability|EndAbility (Utilities|Select :Index _result :Success "Finished" :Blocked "Cancelled" :OffPath "Cancelled" :Aborted "Cancelled" :Invalid "Cancelled")))))

(event EventOnEndAbility
  (params (Reason :type EEndAbilityReason%20Enum :default "Finished"))
  (AI|ClearFocus (Variables|Default|GetAIController)))

(fn ConstructionScript)

(fn AppendDebugStr
  (params (Str :type String))
  (Development|PrintString Str)
  (Variables|Default|SetDebugText (Utilities|String|Append (Variables|Default|GetDebugText) " 
" Str)))

(fn SetAIController
  (bind _aspawn (Utilities|Casting|CastToPawn (Class|AbilityComponent|GetAvatarActor (Class|Ability|GetAbilityComponent))))
  (bind _asaicontroller (Utilities|Casting|CastToAIController (Pawn|GetController _aspawn)))
  (Variables|Default|SetAIController _asaicontroller))