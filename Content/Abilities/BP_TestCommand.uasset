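; Test movement command actor that shows a Cube as an in-world indicator, visible during visualization and when it begins pooled play.
; The move command type, Location or Facing, selects the Cube's indicator material.
; Each visualization tick calls CreateDynamicMaterialInstance, tints the ring with the Selected highlight color and applies proximity fade to ring and pip alpha.
; Follow begin and end events only call the parent; debug prints and highlighting are disconnected.
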(event EventBeginVisualization
  (Rendering|SetActorHiddenInGame false))

(event EventOnMoveCommandTypeChanged
  (params (OldType :type EMoveCommandType%20Enum :default "Location"))
  (Rendering|Material|SetMaterial (Variables|Default|GetCube) 0 (Utilities|Select :Index (Variables|Default|GetType) :Location "/Game/Prototyping/M_CommandIndicator.M_CommandIndicator" :Facing "/Game/Prototyping/MI_DirectionalCommandIndicator.MI_DirectionalCommandIndicator")))

(event EventTick
  (params (DeltaSeconds :type Float%20%28single-precision%29)))

(event EventBeginPlayPooled
  (|CallParentFunction)
  (Rendering|SetActorHiddenInGame false))

(event EventBeginPlay)

(event EventBeginFollowingCommand
  (params (Follower :type Command%20Follower%20Component%20Object%20Reference) (PreviousCommand :type Command%20Object%20Reference))
  (|CallParentFunction Follower PreviousCommand))

(event EventEndFollowingCommand
  (params (Follower :type Command%20Follower%20Component%20Object%20Reference) (NextCommand :type Command%20Object%20Reference))
  (|CallParentFunction Follower NextCommand))

(event EventTickVisualization
  (params (DeltaTime :type Float%20%28single-precision%29))
  (bind _returnvalue (Class|Command|GetProximityFadeOpacity))
  (bind _highlightsettings (Variables|Default|GetHighlightSettings))
  (bind _returnvalue_2 (Class|HighlightSettings|GetHighlightColor _highlightsettings "Selected"))
  (bind _returnvalue_3 (Rendering|Material|CreateDynamicMaterialInstance (Variables|Default|GetCube) 0 0 "None" :!class /Script/Engine.PrimitiveComponent))
  (Rendering|Material|SetVectorParameterValue _returnvalue_3 "RingColor" (Utilities|Struct|MakeLinearColor (.r (.color _returnvalue_2)) (.g (.color _returnvalue_2)) (.b (.color _returnvalue_2)) _returnvalue) :!class /Script/Engine.MaterialInstanceDynamic)
  (bind _returnvalue_4 (Rendering|Material|GetVectorParameterValue _returnvalue_3 "PipColor" :!class /Script/Engine.MaterialInstanceDynamic))
  (Rendering|Material|SetVectorParameterValue _returnvalue_3 "PipColor" (Utilities|Struct|MakeLinearColor (.r _returnvalue_4) (.g _returnvalue_4) (.b _returnvalue_4) _returnvalue) :!class /Script/Engine.MaterialInstanceDynamic))

(event EventEndVisualization
  (Rendering|SetActorHiddenInGame true))

(fn ConstructionScript)