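; Test ability that makes the owning unit shoot its target, using a debug line as the shot visual.
; It focuses the target within a small angle, plays a test montage, then draws a jittered line to it.
; If the target has a UnitStatsComponent, it adds a damage stat modifier with randomized variance from the shooter's stats, then ends after a short delay.
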(event EventOnBeginAbility
  (bind _returnvalue (Class|Ability|GetAbilityComponent))
  (bind _shoottarget (Variables|Default|GetShootTarget))
  (bind _returnvalue_2 (Class|FocusComponent|GetFocusTargetActor _shoottarget))
  (bind _returnvalue_3 (Actor|GetComponentbyClass _returnvalue_2 "/Script/Zombies.UnitStatsComponent"))
  (|FocusTarget "None" (Class|TargetedAbility|GetTarget) "(TagName=\"Focus.Attack\")" 5.0
    (:GainedFocus
      (Animation|Montage|PlayMontage (Class|AbilityComponent|GetSkeletalMeshComponent _returnvalue) "/Game/Characters/Humanoid/Animations/AM_Test.AM_Test"
        (:then
          (Rendering|Debug|DrawDebugLine (Transformation|GetActorLocation (Class|AbilityComponent|GetAvatarActor _returnvalue)) (+ (Transformation|GetActorLocation _returnvalue_2) (* (Math|Random|RandomUnitVector) 2e+01)) "(R=1.000000,G=0.430076,B=0.000000,A=1.000000)" 0.1 3.0)
          (Utilities|IsValid _returnvalue_3
            (:Is%20Valid
              (CallFunction|ApplyDamage _returnvalue_3)
              (Utilities|FlowControl|Delay 0.5)
              (Class|Ability|EndAbility "Finished"))))))))

(fn ConstructionScript)

(fn ApplyDamage
  (params (Target :type Unit%20Stats%20Component%20Object%20Reference))
  (bind _returnvalue (Math|Float|MakeLiteralFloat 1.0))
  (bind _returnvalue_2 (Math|Float|MakeLiteralFloat 0.3))
  (bind _returnvalue_3 (Class|Ability|GetAbilityComponent))
  (bind _returnvalue_4 (Class|AbilityComponent|GetUnitStatsComponent _returnvalue_3))
  (Utilities|IsValid _returnvalue_4
    (:Is%20Valid
      (bind _structout (Utilities|Struct|SetmembersinStatModParams (Class|UnitStatsComponent|MakeStatModParams _returnvalue_4 "/Game/Stats/USM_TestDamage2.USM_TestDamage2") (Utilities|Map|MakeMap "(TagName=\"Magnitude.DamageVariance\")" (Math|Random|RandomFloatinRange (- _returnvalue _returnvalue_2) (+ _returnvalue _returnvalue_2)))))
      (Class|UnitStatsComponent|AddModifier Target _structout))))