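; BP_TestUnitSpawner is a test enemy spawner that maintains up to MaxSpawns live units of SpawnClass.
; BeginPlay starts a Delay loop that calls TrySpawnActor every SpawnRate seconds.
; Each attempt prunes dead units through UnitInterface with a reverse loop, then, if enabled, spawns at a random navigable point within the Sphere radius, raised by HeightOffset.
; Spawned BP_TestEnemyUnit actors receive the MoveTarget component's location as their destination.
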(event EventBeginPlay
  (Utilities|FlowControl|Delay (Variables|Default|GetSpawnRate) :!label _label)
  (CallFunction|TrySpawnActor)
  (goto _label))

(event EventTick
  (params (DeltaSeconds :type Float%20%28single-precision%29)))

(fn ConstructionScript)

(fn TrySpawnActor
  (bind _sphere (Variables|Default|GetSphere))
  (Utilities|FlowControl|Sequence
    (:then_0
      (bind (_arrayindex _arrayelement) (Utilities|Array|ReverseforEachLoop (Variables|Default|GetSpawnedActors))
        (:LoopBody
          (bind _asunit_interface (Utilities|Casting|CastToUnitInterface _arrayelement))
          (if (Class|UnitInterface|IsDead _asunit_interface)
            (Utilities|Array|RemoveIndex (Variables|Default|GetSpawnedActors) _arrayindex)))))
    (:then_1
      (if (and (< (Utilities|Array|Length (Variables|Default|GetSpawnedActors)) (Variables|Default|GetMaxSpawns)) (Variables|Default|GetEnable))
        (if (Utilities|IsValidClass (Variables|Default|GetSpawnClass))
          (bind (_randomlocation _returnvalue) (Class|NavigationSystemV1|GetRandomLocationinNavigableRadius (Transformation|GetWorldLocation _sphere) (Components|Sphere|GetScaledSphereRadius _sphere) 0 0))
          (if _returnvalue
            (bind _returnvalue_2 (Game|SpawnActorfromClass (Variables|Default|GetSpawnClass) (Math|Transform|MakeTransform (+ _randomlocation (Math|Vector|MakeVector 0.0 0.0 (Variables|Default|GetHeightOffset))) "0, 0, 0" "1.000000,1.000000,1.000000") "AdjustIfPossibleButDontSpawnIfColliding" 0 0))
            (Utilities|IsValid _returnvalue_2
              (:Is%20Valid
                (Utilities|Array|Add (Variables|Default|GetSpawnedActors) _returnvalue_2)
                (bind _asbp_test_enemy_unit (Utilities|Casting|CastToBP_TestEnemyUnit _returnvalue_2))
                (Default|SetMoveTarget _asbp_test_enemy_unit true (Transformation|GetWorldLocation (Variables|Default|GetMoveTarget)))))))))))