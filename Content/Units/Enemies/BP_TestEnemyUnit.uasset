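; Test enemy unit that periodically applies a damage stat modifier to nearby player units while alive, using a looping delayed sphere overlap.
; CheckForDeath disables movement, ignores Pawn collision and sets a despawn lifespan, but its health observer registration is unwired here.
; SetMoveTarget writes movement goals to the AI blackboard.
; Fog-of-war events toggle visibility, while a controller arrow follows control rotation and shares highlighting.
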(event Custom|CheckForDeath
  (params (Component :type Unit%20Stats%20Component%20Object%20Reference) (Tag :type Gameplay%20Tag%20Structure) (OldValue :type Unit%20Stat%20Value%20Structure) (NewValue :type Unit%20Stat%20Value%20Structure))
  (bind _charactermovement (Variables|Character|GetCharacterMovement))
  (if (Class|UnitInterface|IsDead)
    (Utilities|FlowControl|DoOnce false :!label _label
      (:Completed
        (Pawn|Components|CharacterMovement|DisableMovement _charactermovement)
        (Components|Activation|Deactivate _charactermovement)
        (Collision|SetCollisionResponsetoChannel (Variables|Default|GetCapsuleComponent) "ECC_Pawn" "ECR_Ignore")
        (Actor|SetLifeSpan 5.0)))
    (else
      (goto _label Reset))))

(event EventBeginPlay
  (Utilities|FlowControl|Delay 0.5 :!label _label)
  (if (not (Class|UnitInterface|IsDead))
    (bind _outactors (Collision|SphereOverlapActors (Transformation|GetActorLocation) 1e+02 (Utilities|Array|MakeArray "ObjectTypeQuery3") "/Script/Zombies.PlayerUnit"))
    (for _array_element _outactors
      (bind _returnvalue (Class|UnitInterface|GetUnitStatsComponent(Message) _array_element))
      (Class|UnitStatsComponent|AddModifier _returnvalue (Class|UnitStatsComponent|MakeStatModParams (Variables|Default|GetUnitStatsComponent) "/Game/Stats/USM_TestDamage.USM_TestDamage")))
    (goto _label)))

(event EventSetHighlighting
  (params (HighlightType :type EHighlightType%20Enum :default "None"))
  (|CallParentFunction HighlightType)
  (Class|HighlightSettings|SetHighlighting (Variables|Default|GetHighlightSettings) (Variables|Default|GetControllerArrow) HighlightType))

(event EventTick
  (params (DeltaSeconds :type Float%20%28single-precision%29))
  (Transformation|SetWorldRotation (Variables|Default|GetControllerArrow) (Pawn|GetControlRotation :!class /Script/Engine.Pawn) false false))

(event EventInitFogOfWarVisibility
  (Rendering|SetActorHiddenInGame true))

(event EventSetFogOfWarVisibletoPawn
  (params (Pawn :type Pawn%20Object%20Reference) (bVisible :type Boolean))
  (Rendering|SetActorHiddenInGame (not bVisible)))

(event EventSetFogOfWarVisibility
  (params (bIsVisible :type Boolean))
  (Rendering|SetActorHiddenInGame (not bIsVisible)))

(fn ConstructionScript)

(fn SetMoveTarget
  (params (bHasMoveTarget :type Boolean) (MoveTarget :type Vector))
  (bind _returnvalue (AI|GetBlackboard 0))
  (AI|Components|Blackboard|SetValueasBool _returnvalue (Utilities|Name|MakeLiteralName "bHasMoveTarget") bHasMoveTarget)
  (AI|Components|Blackboard|SetValueasVector _returnvalue (Utilities|Name|MakeLiteralName "MoveTarget") MoveTarget))