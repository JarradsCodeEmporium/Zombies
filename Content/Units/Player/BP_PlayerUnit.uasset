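; Player unit Blueprint for a tactics game, handling interaction, highlighting, damage numbers and test inventory setup.
; BeginPlay spawns a test item into a free inventory slot, then repeats once after a short delay.
; Stat modifiers applied to the unit spawn floating damage numbers from the Health difference, and highlighting extends to the controller arrow.
; Interact only draws debug text, CanInteract always allows it, and several experiments remain disconnected.
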(event OnSourceInstantaneousModifierApplied(UnitStatsComponent)
  (params (Component :type Unit%20Stats%20Component%20Object%20Reference) (Handle :type Stat%20Mod%20Handle%20Structure%20%28by%20ref%29) (PreviousStats :type Unit%20Stats%20Structure%20%28by%20ref%29) (CurrentStats :type Unit%20Stats%20Structure%20%28by%20ref%29))
  (bind _returnvalue (Components|GetOwner Component))
  (bind _returnvalue_2 (Class|UnitStatsComponent|GetSourceActor Handle))
  (bind (_location _velocity) (CallFunction|GetDamageNumberLocationandVelocity _returnvalue_2 _returnvalue 5e+01 1.5e+03 0.8 0.1))
  (CallFunction|SpawnDamageNumber self _location _velocity 2.0 (Math|Float|Truncate (- (.modifiedvalue (.Value (Utilities|Map|Find (Utilities|Struct|BreakUnitStats PreviousStats) "(TagName=\"Stats.Health\")"))) (.modifiedvalue (.Value (Utilities|Map|Find (Utilities|Struct|BreakUnitStats CurrentStats) "(TagName=\"Stats.Health\")"))))) "/Game/UI/BP_DamageNumber.BP_DamageNumber_C"))

(event EventBeginPlay
  (Utilities|FlowControl|Sequence :!label _label
    (:then_0
      (bind _returnvalue (Game|SpawnActorfromClass "/Game/Items/BP_TestItem.BP_TestItem_C" (Math|Transform|MakeTransform "0, 0, 0" "0, 0, 0" "1.000000,1.000000,1.000000") "Undefined" 0 0))
      (if (Class|InventoryComponent|IsValidLocation (Class|InventoryComponent|FindLocationforItem _returnvalue (Utilities|Struct|MakeInventoryContainerHandle (Variables|Default|GetInventoryComponent) "(TagName=\"Inventory.Test\")")))
        (Class|Item|SetInventoryLocation _returnvalue (Class|InventoryComponent|FindLocationforItem _returnvalue (Utilities|Struct|MakeInventoryContainerHandle (Variables|Default|GetInventoryComponent) "(TagName=\"Inventory.Test\")")))
        (else
          (Development|PrintString "Hello"))))
    (:then_1
      (Utilities|FlowControl|Delay 0.2)
      (Utilities|FlowControl|DoN 1
        (:Exit
          (goto _label))))))

(event EventTick
  (params (DeltaSeconds :type Float%20%28single-precision%29)))

(event EventSetHighlighting
  (params (HighlightType :type EHighlightType%20Enum :default "None"))
  (|CallParentFunction HighlightType)
  (Class|HighlightSettings|SetHighlighting (Variables|Default|GetHighlightSettings) (Variables|Default|GetControllerArrow) HighlightType))

(event EventInteract
  (params (Pawn :type Pawn%20Object%20Reference))
  (Rendering|Debug|DrawDebugString "0, 0,100.000000" "Interact!" self "(R=1.000000,G=0.000000,B=0.830733,A=1.000000)" 2.0)
  (bind _astactics_player_pawn (Utilities|Casting|CastToTacticsPlayerPawn Pawn)))

(fn ConstructionScript)

(fn CanInteract
  (params (Pawn :type Pawn%20Object%20Reference))
  (return true))