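; Debug actor that fills a grid of small cubes covering every custom depth stencil value, for checking stencil-based post-process effects.
; The construction script spawns a 16 by 16 grid of scaled-down cube static mesh components in the actor's local space.
; Each cube renders to custom depth with a unique stencil value derived from its row and column, and has collision disabled.
; The event graph holds no active logic.
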(event EventBeginPlay)

(event Collision|EventActorBeginOverlap
  (params (OtherActor :type Actor%20Object%20Reference)))

(event EventTick
  (params (DeltaSeconds :type Float%20%28single-precision%29)))

(fn ConstructionScript
  (for _index (range 0 15)
    (for _index_2 (range 0 15)
      (bind _returnvalue (AddComponent|AddStaticMeshComponent false (Math|Transform|MakeTransform (* (Math|Vector|MakeVector (Math|Conversions|ToFloat(Integer) _index_2) (Math|Conversions|ToFloat(Integer) _index) 0.0) 3e+01) "0, 0, 0" "0.200000,0.200000,0.200000")))
      (Components|StaticMesh|SetStaticMesh _returnvalue "/Engine/BasicShapes/Cube.Cube")
      (Rendering|SetCustomDepthStencilValue _returnvalue (+ _index_2 (* _index 16)))
      (Rendering|SetRenderCustomDepth _returnvalue true)
      (Collision|SetCollisionEnabled _returnvalue "NoCollision"))))